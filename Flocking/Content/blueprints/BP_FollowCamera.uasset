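; BP_FollowCamera is a follow camera actor that tracks one agent in a flocking simulation.
; Each tick, it snaps to the target agent's location plus an offset and rotates to look at that agent, with no interpolation.
; When the target is invalid, it picks the first agent from the Manager on the FlockingGameModeBase game mode.
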(event Collision|EventActorBeginOverlap
  (params (OtherActor :type Actor%20Object%20Reference)))

(event EventTick
  (params (DeltaSeconds :type Float%20%28single-precision%29))
  (if (Utilities|IsValid (Variables|Components|GetTargetAgent))
    (Transformation|SetActorLocation (+ (Transformation|GetActorLocation (Variables|Components|GetTargetAgent)) (Variables|Components|GetOffset)) false false)
    (Transformation|SetActorRotation (Math|Rotator|FindLookatRotation (Transformation|GetActorLocation self) (Transformation|GetActorLocation (Variables|Components|GetTargetAgent))))
    (else
      (bind _asflocking_game_mode_base (Utilities|Casting|CastToFlockingGameModeBase (Game|GetGameMode)))
      (Variables|Components|SetTargetAgent (Utilities|Array|Get(acopy) (Class|FlockingManager|GetAgents (Variables|/Script/Flocking.FlockingGameModeBase|GetManager _asflocking_game_mode_base)))))))

(fn ConstructionScript)